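; BP_PatrolRoute defines an enemy patrol path from the points of the PatrolRoute spline.
; IncreasePatrolRoute steps CurIdx by Direction and flips Direction at the first and last spline points, so the route ping-pongs instead of looping.
; GetSplinePointPos returns the world-space location of the spline point at CurIdx.
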(event Custom|IncreasePatrolRoute
  (bind _output_get (Variables|Default|SetCurIdx (+ (Variables|Default|GetCurIdx) (Variables|Default|GetDirection))))
  (if (== _output_get (- (Spline|GetNumberOfSplinePoints (Variables|Default|GetPatrolRoute)) 1))
    (Variables|Default|SetDirection -1)
    (elif (== (Variables|Default|GetCurIdx) 0)
      (Variables|Default|SetDirection 1))))

(fn ConstructionScript)

(fn GetSplinePointPos
  (return (Spline|GetLocationatSplinePoint (Variables|Default|GetPatrolRoute) (Variables|Default|GetCurIdx) "World")))