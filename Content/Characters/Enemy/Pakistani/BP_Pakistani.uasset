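; BP_Pakistani is an enemy character Blueprint that arms itself with an assault rifle when play begins.
; After the parent BeginPlay, SpawnGuns spawns BP_AR and snaps it to the WeaponSocket on the Mesh.
; Tick and overlap events are disabled, and unwired leftover nodes reference AloyRef, a bow socket attachment and hiding the actor.
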(event EventBeginPlay
  (|CallParentFunction)
  (CallFunction|SpawnGuns))

(event Collision|EventActorBeginOverlap
  (params (OtherActor :type Actor%20Object%20Reference))
  (|CallParentFunction OtherActor) ; This node is disabled and will not be called.\nDrag off pins to build functionality.
)

(event EventTick
  (params (DeltaSeconds :type Float%20%28single-precision%29))
  (|CallParentFunction DeltaSeconds) ; This node is disabled and will not be called.\nDrag off pins to build functionality.
)

(fn ConstructionScript
  (|CallParentFunction))

(fn SpawnGuns
  (bind _returnvalue (Game|SpawnActorfromClass "/Game/Weapons/BP_AR.BP_AR_C" (Math|Transform|MakeTransform "0, 0, 0" "0, 0, 0" "1.000000,1.000000,1.000000") "Undefined" "MultiplyWithRoot" 0 0))
  (Transformation|AttachComponentToComponent _returnvalue (Variables|Character|GetMesh) "WeaponSocket" "SnapToTarget" "SnapToTarget" "SnapToTarget" true))