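; Human character Blueprint that handles a temporary ragdoll-style fall triggered with a barrel position.
; StartRagdoll turns the actor toward the barrel, then RagdollPrep disables input and sets Falling movement and Ragdoll mesh collision.
; AdjustFlyTime picks a shorter delay at greater barrel distance, after which a looping per-frame timer polls for landing.
; On landing, a montage plays before collision and input are restored.
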(event Custom|StopRagdoll
  (Variables|Default|SetRagdolling? false)
  (bind _returnvalue (Animation|PlayAnimMontage 0 1.0 "None"))
  (Utilities|FlowControl|Delay _returnvalue)
  (CallFunction|RagdollPrep))

(event Custom|StartRagdoll
  (params (BarrelPos :type Vector))
  (if (not (Variables|Default|GetRagdolling?))
    (Variables|Default|SetRagdolling? true)
    (Transformation|SetActorRotation (Math|Interpolation|RInterpTo (Transformation|GetActorRotation) (Math|Rotator|FindLookatRotation (Transformation|GetActorLocation) BarrelPos) (Utilities|Time|GetWorldDeltaSeconds) 0.0))
    (CallFunction|RagdollPrep)
    (CallFunction|AdjustFlyTime BarrelPos)
    (Utilities|FlowControl|Delay (Variables|Default|GetAirTime))
    (bind _returnvalue (Utilities|Time|SetTimerbyEvent (delegate Custom|GetFalling?) (Utilities|Time|GetWorldDeltaSeconds) true))
    (if (not (AI|Components|NavMovement|IsFalling (Variables|Character|GetCharacterMovement)))
      (Utilities|Time|ClearandInvalidateTimerbyHandle _returnvalue)
      (CallFunction|StopRagdoll))))

(event Custom|GetFalling?
  (if (not (AI|Components|NavMovement|IsFalling (Variables|Character|GetCharacterMovement)))
    (Utilities|Time|ClearandInvalidateTimerbyHandle (stale Custom|StartRagdoll _returnvalue))
    (CallFunction|StopRagdoll)))

(event EventBeginPlay)

(event Collision|EventActorBeginOverlap
  (params (OtherActor :type Actor%20Object%20Reference)))

(event EventTick
  (params (DeltaSeconds :type Float%20%28single-precision%29)))

(fn ConstructionScript)

(fn RagdollPrep
  (if (Variables|Default|GetRagdolling?)
    (Input|DisableInput 0)
    (Pawn|Components|CharacterMovement|SetMovementMode (Variables|Character|GetCharacterMovement) "MOVE_Falling" 0)
    (Collision|SetCollisionProfileName (Variables|Character|GetMesh) "Ragdoll" true :!class /Script/Engine.PrimitiveComponent)
    (Variables|Default|SetRagdollStarted? true)
    (else
      (Collision|SetCollisionProfileName (Variables|Character|GetMesh) "CharacterMesh" true :!class /Script/Engine.PrimitiveComponent)
      (Input|EnableInput 0)
      (Variables|Default|SetRagdollStarted? false))))

(fn AdjustFlyTime
  (params (NewParam :type Vector))
  (bind _returnvalue (Transformation|GetActorLocation))
  (bind _returnvalue_2 (Math|Vector|Distance(Vector) _returnvalue NewParam))
  (if (> _returnvalue_2 1.15e+04)
    (if (> _returnvalue_2 1.17e+04)
      (Variables|Default|SetAirTime 0.15)
      (else
        (Variables|Default|SetAirTime 0.25)))
    (else
      (Variables|Default|SetAirTime 0.5))))